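; BP_Movable is an actor with wandering logic confined to a rectangular area, though much of it is unwired.
; On hitting anything except ThirdPersonCharacter, it turns toward a random point in a box and takes a swept forward step.
; A Move event picks a random reachable nearby point and calls AIMoveTo, with no visible link to that point.
; Tick is empty, and the 2D boundary check that would choose between stepping and turning never runs.
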(event Custom|Move
  (Variables|Default|SetTargetLocation (.RandomLocation (AI|Navigation|GetRandomReachablePointinRadius (Transformation|GetActorLocation) 5e+02 0 0)))
  (AI|AIMoveTo 0 "0, 0, 0" 0 5.0 false))

(event EventBeginPlay)

(event Collision|EventHit
  (params (MyComp :type Primitive%20Component%20Object%20Reference) (Other :type Actor%20Object%20Reference) (OtherComp :type Primitive%20Component%20Object%20Reference) (bSelfMoved :type Boolean) (HitLocation :type Vector :default "0, 0, 0") (HitNormal :type Vector :default "0, 0, 0") (NormalImpulse :type Vector :default "0, 0, 0") (Hit :type Hit%20Result%20Structure%20%28by%20ref%29))
  (bind _returnvalue (Transformation|GetActorForwardVector))
  (bind _returnvalue_2 (Transformation|GetActorLocation))
  (bind _speed (Variables|Default|GetSpeed))
  (bind _returnvalue_3 (* _returnvalue _speed))
  (bind _returnvalue_4 (+ _returnvalue_3 _returnvalue_2))
  (Utilities|Casting|CastToThirdPersonCharacter Other
    (:CastFailed
      (Transformation|SetActorRotation (Math|Rotator|FindLookatRotation _returnvalue_4 (Math|Random|RandomPointinBoundingBox "0.000000,0.000000,71.000000" (Math|Vector|MakeVector (Variables|Default|GetMax%20X) (Variables|Default|GetMin%20Y) 0.0))))
      (Transformation|SetActorLocation _returnvalue_4 true false))))

(event EventTick
  (params (DeltaSeconds :type Float%20%28single-precision%29)))

(fn ConstructionScript)

(fn IsActorinBoundaries2D
  (params (Min%20X :type Float%20%28double-precision%29) (Max%20X :type Float%20%28double-precision%29) (Min%20Y :type Float%20%28double-precision%29) (Max%20Y :type Float%20%28double-precision%29))
  (bind _returnvalue (Transformation|GetActorLocation))
  (return (and (Math|Float|InRange(Float) (.x _returnvalue) Min%20X Max%20X) (Math|Float|InRange(Float) (.y _returnvalue) Min%20Y Max%20Y))))