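; BP_Pawn is an AI pawn that wanders endlessly across the navmesh.
; From BeginPlay, Move picks a random reachable point within a radius averaged from the NavMesh bounds' X and Y extents, then calls AIMoveTo and repeats on success or failure.
; Hitting a StaticMeshActor snaps its rotation toward a random point in a navmesh-sized box at a fixed center and calls Move again.
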(event Custom|Move
  (bind _navmesh (Variables|Default|GetNavMesh))
  (bind _boxextent (Collision|GetActorBounds _navmesh false false))
  (bind _output_get (Variables|Default|SetTargetLocation (.RandomLocation (AI|Navigation|GetRandomReachablePointinRadius (Transformation|GetActorLocation) (/ (+ (.x _boxextent) (.y _boxextent)) 2.0) 0 0))))
  (AI|AIMoveTo self _output_get 0 5.0 false
    (:OnSuccess
      _)
    (:OnFail
      _))
  (CallFunction|Move))

(event EventBeginPlay
  (CallFunction|Move))

(event Collision|EventHit
  (params (MyComp :type Primitive%20Component%20Object%20Reference) (Other :type Actor%20Object%20Reference) (OtherComp :type Primitive%20Component%20Object%20Reference) (bSelfMoved :type Boolean) (HitLocation :type Vector :default "0, 0, 0") (HitNormal :type Vector :default "0, 0, 0") (NormalImpulse :type Vector :default "0, 0, 0") (Hit :type Hit%20Result%20Structure%20%28by%20ref%29))
  (bind _navmesh (Variables|Default|GetNavMesh))
  (bind _boxextent (Collision|GetActorBounds _navmesh false false))
  (Utilities|Casting|CastToStaticMeshActor Other)
  (Transformation|SetActorRotation (Math|Rotator|FindLookatRotation (Transformation|GetActorLocation) (Math|Random|RandomPointinBoundingBox "0.000000,0.000000,71.000000" (Math|Vector|MakeVector (.x _boxextent) (.y _boxextent) 0.0))))
  (CallFunction|Move))

(fn ConstructionScript)